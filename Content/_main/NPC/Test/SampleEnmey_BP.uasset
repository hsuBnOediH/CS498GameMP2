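; Test enemy NPC character that takes damage, dies, and punches the player when in range.
; Any damage spawns an explosion at the head and lowers HP, pausing movement for a random hit montage, or playing a random death montage before destroying the actor.
; Player overlap with its sphere starts a punch loop that applies damage mid-montage until the player leaves or dies.
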(event `self.ReceiveBeginPlay`)

(event `self.ReceiveAnyDamage`
  (params (Damage :type "Float (single-precision)") (DamageType :type "DamageType Object Reference") (InstigatedBy :type "Controller Object Reference") (DamageCauser :type "Actor Object Reference"))
  (if (not (`self.Is Dead?`))
    (`|SpawnActorFromClass` "/Game/_main/NPC/Mortar/Expolosion_Bp.Expolosion_Bp_C" (`SceneComponent.K2_GetComponentToWorld` (`self.head`)) "Undefined" "OverrideRootScale" null null)
    (bind _output_get (set `self.HP Cur` (`KismetMathLibrary.FClamp` (- (`self.HP Cur`) Damage) 0.0 100.0)))
    (if (== _output_get 0.0)
      (`CharacterMovementComponent.DisableMovement` (`self.CharacterMovement`))
      (set `self.Is Dead?` true)
      (bind _returnvalue (`self.PlayAnimMontage` (select `int` (`KismetMathLibrary.RandomInteger` 3) :`0` "/Game/_main/NPC/Test/Animation/Death_1_Montage.Death_1_Montage" :`1` "/Game/_main/NPC/Test/Animation/Death_2_Montage.Death_2_Montage" :`2` "/Game/_main/NPC/Test/Animation/Death_3_Montage.Death_3_Montage" :`3` "/Game/_main/NPC/Test/Animation/Death_4_Montage.Death_4_Montage" :!type "AnimMontage Object Reference")))
      (`PrimitiveComponent.SetCollisionEnabled` (`self.CapsuleComponent`) "NoCollision")
      (`KismetSystemLibrary.Delay` _returnvalue)
      (`self.K2_DestroyActor`)
      (else
        (`CharacterMovementComponent.DisableMovement` (`self.CharacterMovement`))
        (bind _returnvalue_2 (`self.PlayAnimMontage` (select `int` (`KismetMathLibrary.RandomInteger` 3) :`0` "/Game/_main/NPC/Test/Animation/Hit_1_Montage.Hit_1_Montage" :`1` "/Game/_main/NPC/Test/Animation/Hit_2_Montage.Hit_2_Montage" :`2` "/Game/_main/NPC/Test/Animation/Hit_3_Montage.Hit_3_Montage" :`3` "/Game/_main/NPC/Test/Animation/Hit_4_Montage.Hit_4_Montage" :!type "AnimMontage Object Reference")))
        (`KismetSystemLibrary.Delay` _returnvalue_2)
        (if (not (`self.Is Dead?`))
          (`CharacterMovementComponent.SetMovementMode` (`self.CharacterMovement`) "MOVE_Walking" 0))))))

(event `self.Sphere.OnComponentBeginOverlap`
  (params (OverlappedComponent :type "PrimitiveComponent Object Reference") (OtherActor :type "Actor Object Reference") (OtherComp :type "PrimitiveComponent Object Reference") (OtherBodyIndex :type Integer) (bFromSweep :type Boolean) (SweepResult :type "HitResult Structure (by ref)"))
  (bind _asue_4asp_character_local (cast `/Game/_main/Character/Ue4ASP_Character_Local` OtherActor))
  (if (not (`/Game/_main/Character/Ue4ASP_Character_Local.Is Dead` _asue_4asp_character_local))
    (set `self.Hit Player` true)
    (bind _returnvalue (`self.PlayAnimMontage` "/Game/_main/NPC/Test/Animation/Punching_0_Montage.Punching_0_Montage" :!label _label))
    (bind _returnvalue_2 (/ _returnvalue 2.0))
    (`KismetSystemLibrary.Delay` _returnvalue_2)
    (if (`self.Hit Player`)
      (if (not (`/Game/_main/Character/Ue4ASP_Character_Local.Is Dead` _asue_4asp_character_local))
        (`GameplayStatics.ApplyDamage` _asue_4asp_character_local 10.0 null self)
        (`KismetSystemLibrary.Delay` _returnvalue_2)
        (goto _label)))))

(event `self.Sphere.OnComponentEndOverlap`
  (params (OverlappedComponent :type "PrimitiveComponent Object Reference") (OtherActor :type "Actor Object Reference") (OtherComp :type "PrimitiveComponent Object Reference") (OtherBodyIndex :type Integer))
  (set `self.Hit Player` false))

(fn `UserConstructionScript`)