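; B2 bomber NPC that shuttles between two marker points while dropping projectiles, and can be destroyed by damage.
; Every five seconds it swaps destination, and a self-rescheduling timer eases its Sphere toward the target by a fixed lerp fraction per tick.
; A separate delay loop spawns a B2_Bullet_BP at BoomREF1 every second.
; Each hit spawns an explosion and lowers HP, destroying the actor at zero.
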(event `self.ReceiveAnyDamage`
  (params (Damage :type "Float (single-precision)") (DamageType :type "DamageType Object Reference") (InstigatedBy :type "Controller Object Reference") (DamageCauser :type "Actor Object Reference"))
  (if (not (`self.Is Dead?`))
    (`|SpawnActorFromClass` "/Game/_main/NPC/Mortar/Expolosion_Bp.Expolosion_Bp_C" (`SceneComponent.K2_GetComponentToWorld` (`self.Sphere`)) "Undefined" "OverrideRootScale" null null)
    (bind _output_get (set `self.HP Cur` (`KismetMathLibrary.FClamp` (- (`self.HP Cur`) Damage) 0.0 100.0)))
    (if (== _output_get 0.0)
      (`self.K2_DestroyActor`))))

(event `self.ReceiveBeginPlay`
  (`self.FindNextLocation`)
  (`self.Relase Boom`))

(event `Moving`
  (bind _sphere (`self.Sphere`))
  (set `self.Alpha` 0.0)
  (`KismetSystemLibrary.K2_SetTimerDelegate` (delegate `Moving`) 0.04)
  (set `self.Alpha` (+ (`self.Alpha`) 0.02))
  (`SceneComponent.K2_SetWorldLocation` _sphere (`KismetMathLibrary.VLerp` (`SceneComponent.K2_GetComponentLocation` _sphere) (`self.Dest Localtion`) (`self.Alpha`)) false false))

(event `FindNextLocation`
  (bind _returnvalue (`SceneComponent.K2_GetComponentLocation` (`self.Dest0`)))
  (set `self.Delta Rotation Z (Yaw)` (`KismetMathLibrary.RandomFloatInRange` -2.0 2.0))
  (if (== (`self.Dest Localtion`) _returnvalue)
    (set `self.Dest Localtion` (`SceneComponent.K2_GetComponentLocation` (`self.Dest1`)))
    (else
      (set `self.Dest Localtion` _returnvalue)))
  (`self.Moving`)
  (`KismetSystemLibrary.Delay` 5.0)
  (`self.FindNextLocation`))

(event `Relase Boom`
  (`|SpawnActorFromClass` "/Game/_main/NPC/B2/B2_Bullet_BP.B2_Bullet_BP_C" (`SceneComponent.K2_GetComponentToWorld` (`self.Boom REF1`)) "Undefined" "OverrideRootScale" null null)
  (`KismetSystemLibrary.Delay` 1.0)
  (`self.Relase Boom`))

(fn `UserConstructionScript`)