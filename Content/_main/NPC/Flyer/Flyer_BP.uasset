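; Flyer NPC that roams between destination points, fires at the player and explodes on taking damage, destroyed at zero HP.
; A random destination and spin are picked every five seconds, and a looping timer eases the sphere toward it by repeated lerp.
; Tick diverts it to a separate point when the player is near and aims an arrow at them.
; Bullets spawn along that aim every two seconds.
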(event `self.ReceiveAnyDamage`
  (params (Damage :type "Float (single-precision)") (DamageType :type "DamageType Object Reference") (InstigatedBy :type "Controller Object Reference") (DamageCauser :type "Actor Object Reference"))
  (if (not (`self.Is Dead?`))
    (`|SpawnActorFromClass` "/Game/_main/NPC/Mortar/Expolosion_Bp.Expolosion_Bp_C" (`SceneComponent.K2_GetComponentToWorld` (`self.Sphere`)) "Undefined" "OverrideRootScale" null null)
    (bind _output_get (set `self.HP Cur` (`KismetMathLibrary.FClamp` (- (`self.HP Cur`) Damage) 0.0 100.0)))
    (if (== _output_get 0.0)
      (`self.K2_DestroyActor`))))

(event `self.ReceiveBeginPlay`
  (`self.FindNextLocation`)
  (`self.Shoot Player`))

(event `Moving`
  (bind _sphere (`self.Sphere`))
  (set `self.Alpha` 0.0)
  (`KismetSystemLibrary.K2_SetTimerDelegate` (delegate `Moving`) 0.04)
  (set `self.Alpha` (+ (`self.Alpha`) 0.02))
  (`SceneComponent.K2_SetWorldLocation` _sphere (`KismetMathLibrary.VLerp` (`SceneComponent.K2_GetComponentLocation` _sphere) (`self.Dest Localtion`) (`self.Alpha`)) false false))

(event `FindNextLocation`
  (set `self.Delta Rotation Z (Yaw)` (`KismetMathLibrary.RandomFloatInRange` -2.0 2.0))
  (set `self.Dest Localtion` (`SceneComponent.K2_GetComponentLocation` (`|GetArrayItem` (`|MakeArray` (`self.Dest1`) (`self.Dest2`) (`self.Dest3`) (`self.Dest4`) (`self.Dest5`) (`self.Dest6`) (`self.Dest0`)) (`KismetMathLibrary.RandomInteger` 6))))
  (`self.Moving`)
  (`KismetSystemLibrary.Delay` 5.0)
  (`self.FindNextLocation`))

(event `self.ReceiveTick`
  (params (DeltaSeconds :type "Float (single-precision)"))
  (`SceneComponent.K2_AddLocalRotation` (`self.Sphere`) (`KismetMathLibrary.MakeRotator` 0.0 0.0 (`self.Delta Rotation Z (Yaw)`)) false false)
  (if (> (`KismetMathLibrary.Vector_Distance` (`SceneComponent.K2_GetComponentLocation` (`Character.Mesh` (`GameplayStatics.GetPlayerCharacter` 0))) (`SceneComponent.K2_GetComponentLocation` (`self.Sphere`))) 1000.0)
    (set `self.IsGoodDistance` true)
    (else
      (set `self.IsGoodDistance` false)
      (set `self.Dest Localtion` (`SceneComponent.K2_GetComponentLocation` (`self.Dest7`)))))
  (`self.LookPlayer`))

(event `LookPlayer`
  (bind _arrow (`self.Arrow`))
  (`SceneComponent.K2_SetWorldRotation` _arrow (`KismetMathLibrary.FindLookAtRotation` (`SceneComponent.K2_GetComponentLocation` _arrow) (`SceneComponent.K2_GetComponentLocation` (`Character.CapsuleComponent` (`GameplayStatics.GetPlayerCharacter` 0)))) false false))

(event `Shoot Player`
  (bind (_returnvalue_location _returnvalue_rotation) (`KismetMathLibrary.BreakTransform` (`SceneComponent.K2_GetComponentToWorld` (`self.Arrow`))))
  (`|SpawnActorFromClass` "/Game/_main/NPC/Flyer/Flyer_Bullet_BP.Flyer_Bullet_BP_C" (`KismetMathLibrary.MakeTransform` (`SceneComponent.K2_GetComponentLocation` (`self.REF`)) _returnvalue_rotation (0.2 0.2 0.2)) "Undefined" "OverrideRootScale" null null)
  (`KismetSystemLibrary.Delay` 2.0)
  (`self.Shoot Player`))

(fn `UserConstructionScript`)