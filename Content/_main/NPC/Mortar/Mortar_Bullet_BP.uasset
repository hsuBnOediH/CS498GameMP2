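; Mortar projectile actor for NPC mortars that reacts to contacts on its sphere collision.
; On overlap, it applies fixed damage only when the touched component is one tagged "Head" on the other actor, printing that component's name, and destroys itself on any overlap.
; On a blocking hit, it spawns an explosion actor at the sphere's location and destroys itself.
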(event `self.Sphere.OnComponentBeginOverlap`
  (params (OverlappedComponent :type "PrimitiveComponent Object Reference") (OtherActor :type "Actor Object Reference") (OtherComp :type "PrimitiveComponent Object Reference") (OtherBodyIndex :type Integer) (bFromSweep :type Boolean) (SweepResult :type "HitResult Structure (by ref)"))
  (for _array_element (`self.GetComponentsByTag` OtherActor "/Script/Engine.ActorComponent" "Head")
    (if (== OtherComp _array_element)
      (`KismetSystemLibrary.PrintString` (`KismetSystemLibrary.GetDisplayName` _array_element))
      (`GameplayStatics.ApplyDamage` OtherActor 20.0 null self)
      (`self.K2_DestroyActor`)))
  (`self.K2_DestroyActor`))

(event `self.Sphere.OnComponentHit`
  (params (HitComponent :type "PrimitiveComponent Object Reference") (OtherActor :type "Actor Object Reference") (OtherComp :type "PrimitiveComponent Object Reference") (NormalImpulse :type "Vector Structure") (Hit :type "HitResult Structure (by ref)"))
  (`|SpawnActorFromClass` "/Game/_main/NPC/Mortar/Expolosion_Bp.Expolosion_Bp_C" (`KismetMathLibrary.Conv_VectorToTransform` (`SceneComponent.K2_GetComponentLocation` (`self.Sphere`))) "Undefined" "OverrideRootScale" null null)
  (`self.K2_DestroyActor`))

(fn `UserConstructionScript`)