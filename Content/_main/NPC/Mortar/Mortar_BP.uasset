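; Mortar NPC that fires projectiles in random directions and can be destroyed by damage.
; From BeginPlay, ShootRandom spawns a scaled-down Mortar_Bullet_BP at the Scene component with random pitch and yaw, then calls itself after a short delay.
; While not dead, each hit spawns an explosion at the Cone and lowers health, destroying the actor at zero.
; Overlapping the Cone applies slight damage to a living Ue4ASP_Character_Local.
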(event `self.ReceiveBeginPlay`
  (`self.ShootRandom`))

(event `ShootRandom`
  (`|SpawnActorFromClass` "/Game/_main/NPC/Mortar/Mortar_Bullet_BP.Mortar_Bullet_BP_C" (`KismetMathLibrary.MakeTransform` (`SceneComponent.K2_GetComponentLocation` (`self.Scene`)) (`KismetMathLibrary.MakeRotator` 0.0 (`KismetMathLibrary.RandomFloatInRange` 0.0 90.0) (`KismetMathLibrary.RandomFloatInRange` -90.0 90.0)) (0.2 0.2 0.2)) "Undefined" "OverrideRootScale" null null)
  (`KismetSystemLibrary.Delay` 2.0)
  (`self.ShootRandom`))

(event `self.ReceiveAnyDamage`
  (params (Damage :type "Float (single-precision)") (DamageType :type "DamageType Object Reference") (InstigatedBy :type "Controller Object Reference") (DamageCauser :type "Actor Object Reference"))
  (if (not (`self.Is Dead?`))
    (`|SpawnActorFromClass` "/Game/_main/NPC/Mortar/Expolosion_Bp.Expolosion_Bp_C" (`SceneComponent.K2_GetComponentToWorld` (`self.Cone`)) "Undefined" "OverrideRootScale" null null)
    (bind _output_get (set `self.HP Cur` (`KismetMathLibrary.FClamp` (- (`self.HP Cur`) Damage) 0.0 100.0)))
    (if (== _output_get 0.0)
      (`self.K2_DestroyActor`))))

(event `self.Cone.OnComponentBeginOverlap`
  (params (OverlappedComponent :type "PrimitiveComponent Object Reference") (OtherActor :type "Actor Object Reference") (OtherComp :type "PrimitiveComponent Object Reference") (OtherBodyIndex :type Integer) (bFromSweep :type Boolean) (SweepResult :type "HitResult Structure (by ref)"))
  (bind _asue_4asp_character_local (cast `/Game/_main/Character/Ue4ASP_Character_Local` OtherActor))
  (if (not (`/Game/_main/Character/Ue4ASP_Character_Local.Is Dead` _asue_4asp_character_local))
    (`GameplayStatics.ApplyDamage` _asue_4asp_character_local 1.0 null self)))

(fn `UserConstructionScript`)