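; Health pickup actor that restores a fixed amount of the player's HP when touched.
; Its cube mesh spins by stepping yaw every tick, independent of frame time.
; Overlap with the box casts to Ue4ASP_Character_Local, adds health to HPCur capped at a hardcoded maximum, then destroys the pickup.
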(event `self.ReceiveTick`
  (params (DeltaSeconds :type "Float (single-precision)"))
  (bind _cube (`self.Cube`))
  (bind (_returnvalue_roll _returnvalue_pitch _returnvalue_yaw) (`KismetMathLibrary.BreakRotator` (`SceneComponent.K2_GetComponentRotation` _cube)))
  (`SceneComponent.K2_SetWorldRotation` _cube (`KismetMathLibrary.MakeRotator` 0.0 0.0 (+ _returnvalue_yaw 1.0)) false false))

(event `self.Box.OnComponentBeginOverlap`
  (params (OverlappedComponent :type "PrimitiveComponent Object Reference") (OtherActor :type "Actor Object Reference") (OtherComp :type "PrimitiveComponent Object Reference") (OtherBodyIndex :type Integer) (bFromSweep :type Boolean) (SweepResult :type "HitResult Structure (by ref)"))
  (bind _returnvalue (+ (`/Game/_main/Character/Ue4ASP_Character_Local.HP Cur` (`self.Player REF`)) 20.0))
  (bind _asue_4asp_character_local (cast `/Game/_main/Character/Ue4ASP_Character_Local` OtherActor))
  (set `self.Player REF` _asue_4asp_character_local)
  (`|ExecutionSequence`
    (:`then_0`
      (if (> _returnvalue 100.0)
        (set `/Game/_main/Character/Ue4ASP_Character_Local.HP Cur` 100.0 (`self.Player REF`))
        (else
          (set `/Game/_main/Character/Ue4ASP_Character_Local.HP Cur` _returnvalue (`self.Player REF`)))))
    (:`then_1`
      (`self.K2_DestroyActor`))))

(fn `UserConstructionScript`)