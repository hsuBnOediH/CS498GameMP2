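; Bullet actor for the gun that damages only when it hits a component tagged "Head".
; On sphere overlap it compares the touched component against the other actor's "Head"-tagged components, printing the name and applying damage on a match.
; The bullet destroys itself on any overlap, so non-head hits deal no damage, and otherwise expires after a short delay from spawn.
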(event `self.ReceiveBeginPlay`
  (`KismetSystemLibrary.Delay` 5.0)
  (`self.K2_DestroyActor`))

(event `self.Sphere.OnComponentBeginOverlap`
  (params (OverlappedComponent :type "PrimitiveComponent Object Reference") (OtherActor :type "Actor Object Reference") (OtherComp :type "PrimitiveComponent Object Reference") (OtherBodyIndex :type Integer) (bFromSweep :type Boolean) (SweepResult :type "HitResult Structure (by ref)"))
  (for _array_element (`self.GetComponentsByTag` OtherActor "/Script/Engine.ActorComponent" "Head")
    (if (== OtherComp _array_element)
      (`KismetSystemLibrary.PrintString` (`KismetSystemLibrary.GetDisplayName` _array_element))
      (`GameplayStatics.ApplyDamage` OtherActor 20.0 null self)
      (`self.K2_DestroyActor`)))
  (`self.K2_DestroyActor`))

(fn `UserConstructionScript`)